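; BP_Pawn is the player pawn for a Wordle-style game and forwards keyboard input to the game mode.
; On BeginPlay it casts and caches the wordle game mode.
; An any-key handler passes key display names that pass a letter check to OnLetterTyped, while Backspace and Enter call OnBackspaceTyped and SubmitWord.
; The pawn holds no word logic itself, leaving that to the game mode.
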(event EventBeginPlay
  (bind _aswordlegamemode (Utilities|Casting|CastTowordlegamemode (Game|GetGameMode)))
  (Variables|Default|SetGameMode _aswordlegamemode))

(event Input|KeyboardEvents|AnyKey
  (params (Key :type Key%20Structure :default "None"))
  (bind _returnvalue (Class|KismetInputLibrary|KeyGetDisplayName Key true))
  (bind _returnvalue_2 (Utilities|String|ToString(Text) _returnvalue))
  (:Pressed
    (bind _returnvalue_3 (Class|WordleLibrary|IsLetter _returnvalue_2))
    (if _returnvalue_3
      (Default|OnLetterTyped (Variables|Default|GetGameMode) _returnvalue_2))))

(event Input|KeyboardEvents|Backspace
  (params (Key :type Key%20Structure :default "None"))
  (:Pressed
    (Default|OnBackspaceTyped (Variables|Default|GetGameMode))))

(event Input|KeyboardEvents|Enter
  (params (Key :type Key%20Structure :default "None"))
  (:Pressed
    (Default|SubmitWord (Variables|Default|GetGameMode))))

(fn ConstructionScript)