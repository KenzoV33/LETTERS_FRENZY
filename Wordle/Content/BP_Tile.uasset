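; BP_Tile is a letter tile actor that displays a letter, with error and submit animations, apparently for a word game.
; Front and back Letter_Widget components stay in sync through SetLetter, while GetLetter reads the front one.
; ErrorLetter shakes the Cube sideways via a sped-up timeline.
; SubmitLetter rotates the Cube through a flip timeline, with a timer swapping in the supplied material a quarter of the way through.
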(event Custom|ClearLetter
  (CallFunction|SetLetter))

(event Custom|SetLetter
  (params (Letter :type String))
  (bind _returnvalue (Utilities|Text|ToText(String) Letter))
  (bind _asletter_widget (Utilities|Casting|CastToLetter_Widget (UserInterface|GetUserWidgetObject (Variables|Default|GetWidgetFront))))
  (Default|SetLetter _asletter_widget _returnvalue)
  (bind _asletter_widget_2 (Utilities|Casting|CastToLetter_Widget (UserInterface|GetUserWidgetObject (Variables|Default|GetWidgetBack))))
  (Default|SetLetter _asletter_widget_2 _returnvalue))

(event Custom|ErrorLetter
  (bind _alpha (Timeline|ErrorTimeline PlayFromStart)
    (:Update
      (Transformation|SetRelativeLocation (Variables|Default|GetCube) (Math|Vector|Lerp(Vector) "0.000000,-10.000000,0.000000" "0.000000,10.000000,0.000000" _alpha) false false))))

(event Custom|SubmitLetter
  (params (Material :type Material%20Interface%20Object%20Reference))
  (Utilities|Time|SetTimerbyEvent (delegate Custom|ChangesColors) (/ (Components|Timeline|GetTimelineLength (Variables|Default|GetFlipTimeLine)) 4.0))
  (bind _alpha (Timeline|FlipTimeLine PlayFromStart)
    (:Update
      (Transformation|SetRelativeRotation (Variables|Default|GetCube) (Math|Rotator|Lerp(Rotator) "0.000000,0.000000,0.000000" "0.000000,0.000000,8.000000" _alpha) false false))))

(event Custom|ChangesColors
  (Rendering|Material|SetMaterial (Variables|Default|GetCube) 0 (stale Custom|SubmitLetter Material)))

(event EventBeginPlay
  (Components|Timeline|SetPlayRate (Variables|Default|GetErrorTimeline) 3.0))

(fn ConstructionScript)

(fn GetLetter
  (bind _asletter_widget (Utilities|Casting|CastToLetter_Widget (UserInterface|GetUserWidgetObject (Variables|Default|GetWidgetFront))))
  (return (Utilities|String|ToString(Text) (Default|GetLetter _asletter_widget))))