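; BP_Board is the tile grid for a word-guessing game, with one row per guess and one column per letter.
; On BeginPlay it spawns cleared BP_Tile actors, offset horizontally around BoardTopMiddleLocation and stacked downward by tile size plus padding.
; Tiles live in a flat row-major array, which GetTile indexes by guess and letter.
; It also exposes board dimensions and can destroy itself along with its tiles.
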(event EventBeginPlay
  (CallFunction|InitializeBoard))

(fn ConstructionScript)

(fn DestroyBoardandTiles
  (for _array_element (Variables|Default|GetTiles)
    (Actor|DestroyActor _array_element))
  (Actor|DestroyActor))

(fn InitializeBoard
  (bind _tilesize (Variables|Default|GetTileSize))
  (bind _paddingsize (Variables|Default|GetPaddingSize))
  (bind _returnvalue (+ _tilesize _paddingsize))
  (for _index (range 0 (- (Variables|Default|GetNumGuesses) 1))
    (LocalVariables|SetGuessIndex%20%28local%29 _index)
    (for _index_2 (range 0 (- (Variables|Default|GetWordLength) 1))
      (LocalVariables|SetLetterIndex%20%28local%29 _index_2)
      (bind _returnvalue_2 (Game|SpawnActorfromClass "/Game/BP_Tile.BP_Tile_C" (Math|Transform|MakeTransform (+ (Transformation|GetWorldLocation (Variables|Default|GetBoardTopMiddleLocation)) (Math|Vector|MakeVector 0.0 (* (- (LocalVariables|GetLetterIndex%20%28local%29) (/ (Variables|Default|GetWordLength) 2)) _returnvalue -1.0) (* (LocalVariables|GetGuessIndex%20%28local%29) _returnvalue -1.0))) (Transformation|GetWorldRotation (Variables|Default|GetBoardTopMiddleLocation)) "1.000000,1.000000,1.000000") "Undefined" "MultiplyWithRoot" 0 0))
      (Default|ClearLetter _returnvalue_2)
      (Utilities|Array|Add (Variables|Default|GetTiles) _returnvalue_2))))

(fn GetWordLength
  (return (Variables|Default|GetWordLength)))

(fn GetWordLastValidindex
  (return (- (CallFunction|GetWordLength) 1)))

(fn GetTile
  (params (GuessIndex :type Integer) (LetterIndex :type Integer))
  (return (Utilities|Array|Get(acopy) (Variables|Default|GetTiles) (+ (* GuessIndex (Variables|Default|GetWordLength)) LetterIndex))))

(fn GetNumGuesses
  (return (Variables|Default|GetNumGuesses)))